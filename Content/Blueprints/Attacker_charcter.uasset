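; Attacker character Blueprint that gives its mesh a tinted look for the attacker role.
; The construction script creates a dynamic material instance from SimpleMaterial, sets its Color parameter to a mint green and applies it to the mesh's first material slot.
; The event graph holds only disabled default events, so the Blueprint adds no gameplay logic of its own.
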(fn `UserConstructionScript`
  (`parent.UserConstructionScript`)
  (bind _returnvalue (`KismetMaterialLibrary.CreateDynamicMaterialInstance` "/Game/AdvancedLocomotionV3/Maps/simpleMaterial.simpleMaterial"))
  (bind _output_get (set `self.dynamicMaterial` _returnvalue))
  (`MaterialInstanceDynamic.SetVectorParameterValue` _output_get "Color" (struct :`R` 0.32412 :`G` 1.0 :`B` 0.723001 :`A` 1.0))
  (`PrimitiveComponent.SetMaterial` (`self.Mesh`) 0 (`self.dynamicMaterial`)))