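; Player controller for an ALS-based multiplayer team game, handling team selection, health, death and respawn.
; BeginPlay and respawn possess a StartingCamera on the server and show the team selector; team choice spawns through the game mode, with the HUD created locally.
; Death triggers ragdoll, sound and a delayed respawn, while Comma respawns immediately.
; It also runs a looping jetpack timer counter and copies team counters from the game mode every Tick.
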(event `StartJetpackTimer`
  ;[1 1 1] Jetpack timer eventsd
  (`KismetSystemLibrary.K2_SetTimer` null "JetpackTimers" 0.05 true))

(event `ClearJetpackTimer`
  ;[1 1 1] Jetpack timer eventsd
  (`KismetSystemLibrary.K2_ClearTimer` null "JetpackTimers"))

(event `SetJetpacTimer`
  ;[1 1 1] Jetpack timer eventsd
  (set `self.MaxTime` 100.0)
  (`GameplayStatics.PlaySound2D` "/Game/Sounds/Ready.ready" 1.0 1.0 0.0 null null))

(event `self.ReceiveTick`
  (params (DeltaSeconds :type "Float (single-precision)"))
  (`self.CallForCounterVariables`))

(event `ResetJetpackTimer`
  ;[1 1 1] Jetpack timer eventsd
  (set `self.MaxTime` 0.0))

(event `RespawnViaTeamselect`
  ;[1 1 1] Respawn logic
  (`Widget.SetVisibility` (stale `TeamSelectedCient` _returnvalue) "Hidden" :!label _label)
  (bind _output_get (set `self.PlayerHealth` 35.0))
  (`/Game/UI/PlayerHUD.UpdateHealth_HUD` (`self.PlayerHud`) _output_get)
  (`self.ServerDestroyActors`)
  (`self.OwnerBackToTeamSelect`)
  (`WidgetBlueprintLibrary.SetInputMode_UIOnlyEx` null (stale `TeamSelectedCient` _returnvalue)))

(event `Key|Comma`
  (params (Key :type "Key Structure"))
  (:`Pressed`
    (`self.ClearJetpackTimer`)
    ;[1 1 1] Respawn logic
    (`self.SetJetpacTimer`)
    (goto _label)))

(event `ServerDestroyActors`
  ;[1 1 1] Respawn logic
  ;;[1 1 1] Server destroys actors
  (`self.K2_DestroyActor` (`self.K2_GetPawn`))
  (`self.UnPossess`))

(event `OwnerBackToTeamSelect`
  (`|ExecutionSequence` :!label _label_2
    (:`then_0`
      (`/Engine/EditorBlueprintResources/ActorMacros.Switch Has Authority`
        (:`Authority`
          (bind _outactors (`GameplayStatics.GetAllActorsOfClass` "/Game/pawnsAndShit/StartingCamera.StartingCamera_C"))
          (`self.Possess` (`|GetArrayItem` _outactors)))))
    (:`then_1`
      (if (`self.IsLocalController`)
        (bind _returnvalue (`|GenericCreateObject` "/Game/UI/TeamSelector.TeamSelector_C" (`GameplayStatics.GetPlayerController` 0)))
        (`UserWidget.AddToViewport` _returnvalue 0)
        (set `self.bShowMouseCursor` true)))))

(event `self.ReceiveBeginPlay`
  (goto _label_2))

(event `TeamSelected`
  (params (Team :type "/Game/pawnsAndShit/Teams Enum" :default "NewEnumerator0"))
  (`|ExecutionSequence`
    (:`then_0`
      (`/Game/GameModes/ALS_GameMode_MP.SpawnPlayer` (cast `/Game/GameModes/ALS_GameMode_MP` (`GameplayStatics.GetGameMode`) :!pure true) Team self)
      (`self.CallForCounterVariables`))))

(event `TeamSelectedCient`
  (if (`self.IsLocalController`)
    (bind _returnvalue (`|CreateWidget` "/Game/UI/PlayerHUD.PlayerHUD_C" (`GameplayStatics.GetPlayerController` 0)))
    (bind _output_get (set `self.PlayerHud` _returnvalue))
    (`UserWidget.AddToViewport` _output_get 0)
    (`/Game/UI/PlayerHUD.UpdateHealth_HUD` _output_get (`self.PlayerHealth`))
    (set `self.IsDead` false)))

(event `DamagePlayer`
  (params (Damage :type "Float (double-precision)"))
  (bind _playerhealth (`self.PlayerHealth`))
  (if (<= _playerhealth 0.0)
    (bind _asals_base_character (cast `/Game/Blueprints/ALS_BaseCharacter` (`self.K2_GetPawn`)))
    (`/Game/Blueprints/ALS_BaseCharacter.To_Ragdoll Event` _asals_base_character)
    ;[1 1 1] death sound
    (`/Game/Blueprints/ALS_BaseCharacter.ServerDeathSound` _asals_base_character "/Game/StarterContent/Audio/deathSound01.deathSound01" (`self.K2_GetActorLocation` _asals_base_character))
    ;[1 1 1] go to third person when dead
    (`/Game/Blueprints/ALS_BaseCharacter.Set ALS_ViewMode Event` _asals_base_character "NewEnumerator0")
    ;[1 1 1] set is death variable
    (set `self.IsDead` true)
    ;[1 1 1] hide player hud when dead
    (`Widget.SetVisibility` (stale `TeamSelectedCient` _returnvalue) "Hidden")
    ;[1 1 1] Respawn delay
    (`KismetSystemLibrary.Delay` 2.0)
    (`self.RespawnViaTeamselect`)
    (cast `/Game/Blueprints/ALS_BaseCharacter` (`GameplayStatics.GetPlayerPawn` 0))
    (`self.ClearJetpackTimer`)
    (`self.SetJetpacTimer`)
    (else
      (bind _output_get (set `self.PlayerHealth` (- _playerhealth Damage)))
      (`/Game/UI/PlayerHUD.UpdateHealth_HUD` (`self.PlayerHud`) _output_get))))

(event `CallForCounterVariables`
  ;[1 1 1] Get GameMode team count and add the amount to replicated value
  (bind _asals_game_mode_mp (cast `/Game/GameModes/ALS_GameMode_MP` (`GameplayStatics.GetGameMode`))
    (:`then`
      (set `self.BlöValue` (`/Game/GameModes/ALS_GameMode_MP.CounterBlö` _asals_game_mode_mp))
      (set `self.RödValue` (`/Game/GameModes/ALS_GameMode_MP.CounterRöd` _asals_game_mode_mp)))
    (:`CastFailed`
      (`KismetSystemLibrary.PrintString` "Counter cast failed"))))

(fn `JetpackTimers`
  (set `self.MaxTime` (+ (`self.MaxTime`) 1.0)))

(fn `UserConstructionScript`)