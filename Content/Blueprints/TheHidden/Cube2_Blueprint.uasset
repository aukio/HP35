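; Cube Blueprint that reveals its static mesh while something overlaps its capsule and hides it otherwise.
; Begin overlap on a hidden mesh waits briefly, toggles visibility on, then sets an IsOverlapping flag, which end overlap clears.
; Tick polls that flag and, after the same short delay, toggles a visible mesh off, propagating to child components.
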(event `self.ReceiveTick`
  (params (DeltaSeconds :type "Float (single-precision)"))
  (bind _staticmeshcomponent (`self.StaticMeshComponent`))
  ;[1 1 1] is it visible?
  (if (`SceneComponent.bVisible` _staticmeshcomponent)
    (if (not (`self.IsOverlapping`))
      (`KismetSystemLibrary.Delay` 0.2)
      ;[1 1 1] hide
      (`SceneComponent.ToggleVisibility` _staticmeshcomponent true))))

(event `self.Capsule.OnComponentBeginOverlap`
  (params (OverlappedComponent :type "PrimitiveComponent Object Reference") (OtherActor :type "Actor Object Reference") (OtherComp :type "PrimitiveComponent Object Reference") (OtherBodyIndex :type Integer) (bFromSweep :type Boolean) (SweepResult :type "HitResult Structure (by ref)"))
  (bind _staticmeshcomponent (`self.StaticMeshComponent`))
  ;[1 1 1] is it visible?
  (if (not (`SceneComponent.bVisible` _staticmeshcomponent))
    (`KismetSystemLibrary.Delay` 0.2)
    (`SceneComponent.ToggleVisibility` _staticmeshcomponent true)
    (set `self.IsOverlapping` true)))

(event `self.Capsule.OnComponentEndOverlap`
  (params (OverlappedComponent :type "PrimitiveComponent Object Reference") (OtherActor :type "Actor Object Reference") (OtherComp :type "PrimitiveComponent Object Reference") (OtherBodyIndex :type Integer))
  (set `self.IsOverlapping` false))

(fn `UserConstructionScript`)