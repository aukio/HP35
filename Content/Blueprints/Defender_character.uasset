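; Defender player character that handles a left-click gun attack and tints its mesh red through a dynamic material in the construction script.
; The attack checks a cooldown and the MainPlayerController's dead flag, calls ServerFireGun, then briefly locks both attacks.
; Attack sounds are relayed from server events to multicast events that play at a location.
; A slower secondary attack with the same pattern exists but has no input wired, so never runs.
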(event `Key|LeftMouseButton`
  (params (Key :type "Key Structure"))
  ;[1 1 1] Primary Attack
  (:`Pressed`
    ;;[1 1 1] Attack cooldown check
    (if (`self.AttackCooldown`)
      (set `self.AttackCooldown` false)
      (set `self.SecAttackCooldown` false)
      (bind _asmain_player_controller (cast `/Game/Blueprints/MainPlayerController` (`GameplayStatics.GetPlayerController` 0)))
      ;;[1 1 1] Disable attack if dead
      (if (not (`/Game/Blueprints/MainPlayerController.IsDead` _asmain_player_controller))
        (`self.ServerFireGun` 10.0)
        ;;[1 1 1] Knife sound
        (`self.ServerKnifeSound` "/Game/Sounds/gunshot01.gunshot01")
        ;;[1 1 1] Apply cooldown
        (`KismetSystemLibrary.Delay` 0.15)
        (set `self.AttackCooldown` true)
        (set `self.SecAttackCooldown` true)))))

(event `CustomEvent_1`
  (params (Sound :type "SoundBase Object Reference") (Location :type "Vector Structure"))
  ;[1 1 1] Primary Attack
  ;;[1 1 1] Knife sound
  (`self.MulticastKnifeSound` Sound Location))

(event `CustomEvent`
  (params (Sound :type "SoundBase Object Reference") (Location :type "Vector Structure"))
  ;[1 1 1] Knife sound
  (`GameplayStatics.PlaySoundAtLocation` Sound Location (struct) 1.0 1.0 0.0 null null null))

(event `Key|RightMouseButton`
  (params (Key :type "Key Structure"))
  ;[1 1 1] Secondary attack
)

(event `CustomEvent_3`
  (params (Sound :type "SoundBase Object Reference") (Location :type "Vector Structure"))
  ;[1 1 1] Knife sound
  (`self.MulticastSecKnifeSound` Sound Location))

(event `CustomEvent_2`
  (params (Sound :type "SoundBase Object Reference") (Location :type "Vector Structure"))
  ;[1 1 1] Knife sound
  (`GameplayStatics.PlaySoundAtLocation` Sound Location (struct) 1.0 1.0 0.0 null null null))

(fn `UserConstructionScript`
  (`parent.UserConstructionScript`)
  ;[1 1 1] get the parent material
  (bind _returnvalue (`KismetMaterialLibrary.CreateDynamicMaterialInstance` "/Game/AdvancedLocomotionV3/Maps/simpleMaterial.simpleMaterial"))
  ;[1 1 1] apply random name
  (bind _output_get (set `self.DynamicMaterial` _returnvalue))
  ;[1 1 1] tell which parameter to edit
  (`MaterialInstanceDynamic.SetVectorParameterValue` _output_get "Color" (struct :`R` 1.0 :`G` 0.216748 :`B` 0.186899 :`A` 1.0))
  ;[1 1 1] apply changes
  (`PrimitiveComponent.SetMaterial` (`self.Mesh`) 0 (`self.DynamicMaterial`)))